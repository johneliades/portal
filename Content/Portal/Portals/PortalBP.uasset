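; One half of a linked blue/orange portal pair that shows a live see-through view and teleports Chell and other objects.
; Each tick it mirrors the player camera onto the pair's scene capture, hiding traced blockers.
; Overlaps trigger teleports that rotate view or velocity, with an ignore list preventing bounce-back.
; SpawnPortal nudges placement until four edge planes fit one surface, else reverts, while a timeline scales opening and closing.
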(event OnComponentBeginOverlap(Collission)
  (params (OverlappedComponent :type Primitive%20Component%20Object%20Reference) (OtherActor :type Actor%20Object%20Reference) (OtherComp :type Primitive%20Component%20Object%20Reference) (OtherBodyIndex :type Integer) (bFromSweep :type Boolean) (SweepResult :type Hit%20Result%20Structure%20%28by%20ref%29))
  ;[1 1 1] Teleportation
  (CallFunction|BeginTeleportation OtherActor OtherComp))

(event OnComponentEndOverlap(Collission)
  (params (OverlappedComponent :type Primitive%20Component%20Object%20Reference) (OtherActor :type Actor%20Object%20Reference) (OtherComp :type Primitive%20Component%20Object%20Reference) (OtherBodyIndex :type Integer))
  ;[1 1 1] Teleportation
  (Utilities|Array|RemoveItem (Variables|Default|GetTemporary%20Ignore%20List) OtherActor))

(event Custom|Show
  (bind _pair_portal (Variables|Default|GetPair%20Portal))
  (bind _portal (Variables|Default|GetPortal))
  (bind _attenuation (Variables|Default|GetAttenuation))
  (bind _portal_2 (Variables|Default|GetPortal))
  (bind _returnvalue (Transformation|GetWorldLocation _portal))
  ;[1 1 1] Show-Hide Portals
  (Components|Timeline|SetPlayRate (Variables|Default|GetResize) 1.0)
  (Variables|Default|SetResizing true)
  (Rendering|SetVisibility _portal_2 true false)
  (Rendering|SetVisibility (Variables|Default|GetDefaultSceneRoot) true false)
  ;;[1 1 1] Teleport Already colliding actors
  (for _array_element (Collision|GetOverlappingActors (Variables|Default|GetCollission) "/Script/Engine.Actor" :!class /Script/Engine.PrimitiveComponent)
    (CallFunction|BeginTeleportation _array_element))
  (for _array_element_2 (Collision|GetOverlappingActors (Variables|PortalBP_C|GetCollission _pair_portal) "/Script/Engine.Actor" :!class /Script/Engine.PrimitiveComponent)
    (CallFunction|BeginTeleportation _pair_portal _array_element_2))
  (if (Variables|Default|GetIsBlue)
    (Audio|PlaySoundatLocation "/Game/Portal/Portals/Audio/portal_open1.portal_open1" _returnvalue "0, 0, 0" 1.0 1.0 0.0 _attenuation 0 0)
    (bind (_direction _alpha) (Timeline|Resize PlayFromStart)
      (:Update
        (Transformation|SetWorldScale3D _portal_2 (Math|Vector|Lerp(Vector) "0.100000,0.100000,0.100000" "2.500000,1.000000,2.000000" _alpha)))
      (:Finished
        (Variables|Default|SetResizing false)
        (switch Utilities|FlowControl|Switch|SwitchonETimelineDirection _direction
          (:Backward
            (Rendering|SetVisibility _portal_2 false false)))))
    (else
      (Audio|PlaySoundatLocation "/Game/Portal/Portals/Audio/portal_open2.portal_open2" _returnvalue "0, 0, 0" 1.0 1.0 0.0 _attenuation 0 0)
      (Timeline|Resize PlayFromStart))))

(event Custom|BeginTeleportation
  (params (Actor :type Actor%20Object%20Reference) (Component :type Primitive%20Component%20Object%20Reference))
  (bind _chell (Variables|Default|GetChell))
  (bind _pair_portal (Variables|Default|GetPair%20Portal))
  (bind _pair_portal_2 (Variables|Default|GetPair%20Portal))
  (bind _portal (Variables|PortalBP_C|GetPortal _pair_portal))
  (bind _returnvalue (Transformation|GetWorldLocation _portal))
  ;[1 1 1] Teleportation
  (if (Math|Boolean|ANDBoolean (Rendering|IsVisible (Variables|Default|GetPortal self)) (Rendering|IsVisible (Variables|PortalBP_C|GetPortal _pair_portal_2)) (not (Utilities|Array|ContainsItem (Variables|Default|GetTemporary%20Ignore%20List) Actor)))
    (Utilities|Array|Add (Variables|PortalBP_C|GetTemporary%20Ignore%20List _pair_portal_2) Actor)
    (bind _aschell (Utilities|Casting|CastToChell Actor)
      (:then
        (bind (_location _impactrotation _portalrotation) (CallFunction|CalculatePortalRotation (Variables|/Script/Engine.PlayerCameraManager|GetTransformComponent (Game|GetPlayerCameraManager 0))))
        (Default|Teleport _aschell _returnvalue _impactrotation _portalrotation)
        (bind _alpha (Timeline|Timeline_0 PlayFromStart)
          (:Update
            (Pawn|SetControlRotation (Pawn|GetController (Game|GetInstigator _aschell)) (Math|Rotator|Lerp(Rotator) _impactrotation (Math|Rotator|MakeRotator 0.5 (.Pitch (Math|Rotator|BreakRotator _impactrotation)) (.Yaw (Math|Rotator|BreakRotator _impactrotation))) _alpha true)))
          (:Finished
            (if (Variables|/Game/Portal/FPC/Chell.Chell_C|GetHoldingObject _chell) :!label _label
              (Physics|Components|PhysicsHandle|ReleaseComponent (Variables|/Game/Portal/FPC/Chell.Chell_C|GetPhysicsHandle _chell))
              (Variables|/Game/Portal/FPC/Chell.Chell_C|SetHoldingObject (Variables|Default|GetChell) false)))))
      (:CastFailed
        (bind (_location_2 _impactrotation_2 _portalrotation_2) (CallFunction|CalculatePortalRotation Component))
        (Transformation|SetWorldLocationAndRotation Component _returnvalue _impactrotation_2 false false)
        (Physics|SetPhysicsLinearVelocity Component (Math|Vector|RotateVector (Transformation|GetComponentVelocity Component) _portalrotation_2) false "None")
        (goto _label)))))

(event Custom|Hide
  (bind _portal (Variables|Default|GetPortal))
  ;[1 1 1] Show-Hide Portals
  (Components|Timeline|SetPlayRate (Variables|Default|GetResize) (Variables|Default|GetDespawnRate))
  (Rendering|SetVisibility (Variables|Default|GetDefaultSceneRoot) false false)
  (bind (_direction _alpha) (Timeline|Resize ReverseFromEnd)
    (:Update
      (Transformation|SetWorldScale3D _portal (Math|Vector|Lerp(Vector) "0.100000,0.100000,0.100000" "2.500000,1.000000,2.000000" _alpha)))
    (:Finished
      (Variables|Default|SetResizing false)
      (switch Utilities|FlowControl|Switch|SwitchonETimelineDirection _direction
        (:Backward
          (Rendering|SetVisibility _portal false false))))))

(event EventBeginPlay
  ;[1 1 1] Initialisation
  (Variables|Default|SetBackup%20Capture%20Material (Rendering|Material|GetMaterial (Variables|Default|GetPortal) 1)))

(event EventTick
  (params (DeltaSeconds :type Float%20%28single-precision%29))
  (bind _portal (Variables|Default|GetPortal))
  (bind _pair_portal (Variables|Default|GetPair%20Portal))
  (bind _pair_portal_2 (Variables|Default|GetPair%20Portal))
  (bind _portalcapture (Variables|PortalBP_C|GetPortalCapture _pair_portal))
  ;[1 1 1] Check if Target-Pair Portal "exists"
  (if (and (Rendering|IsVisible (Variables|PortalBP_C|GetPortal _pair_portal_2)) (not (Variables|PortalBP_C|GetResizing _pair_portal_2)))
    (Utilities|FlowControl|Sequence
      (:then_0
        (goto _label Reset))
      (:then_1
        ;[1 1 1] Render Current Portal
        (bind (_location _impactrotation) (CallFunction|CalculatePortalRotation (Variables|/Script/Engine.PlayerCameraManager|GetTransformComponent (Variables|/Script/Engine.PlayerController|GetPlayerCameraManager (Game|GetPlayerController 0)))))
        (Transformation|SetWorldLocationAndRotation (Variables|PortalBP_C|GetPortalCapture (Variables|Default|GetPair%20Portal)) _location _impactrotation false false)
        (Rendering|Material|SetMaterial (Variables|Default|GetPortal) 1 (Variables|Default|GetBackup%20Capture%20Material))
        ;[0.9705 1 0] Hide walls between target-pair portal and its camera
        (Class|SceneCaptureComponent|ClearHiddenComponents _portalcapture)
        (bind (_outhits _returnvalue) (Class|KismetSystemLibrary|CapsuleTraceMultiforObjects (Transformation|GetWorldLocation _portalcapture) (Transformation|GetWorldLocation (Variables|PortalBP_C|GetPortal _pair_portal)) 0.0 0.0 (Variables|Default|GetObjectsType) false 0 "None" true))
        (if _returnvalue
          (for _array_element _outhits
            (Class|SceneCaptureComponent|HideActorComponents _portalcapture (Components|GetOwner (.HitComponent (Collision|BreakHitResult _array_element))) true)))))
    (else
      (Utilities|FlowControl|DoOnce false :!label _label
        (:Completed
          (if (Variables|Default|GetIsBlue)
            (Rendering|Material|SetMaterial _portal 1 "/Game/Portal/Portals/Empty/MagicBall_Blue.MagicBall_Blue")
            (else
              (Rendering|Material|SetMaterial _portal 1 "/Game/Portal/Portals/Empty/MagicBall_oRANGE.MagicBall_Orange"))))))))

(fn ConstructionScript)

(fn CalculatePortalRotation
  (params (Component :type Scene%20Component%20Object%20Reference))
  (bind _pair_portal (Variables|Default|GetPair%20Portal))
  (bind _portal (Variables|Default|GetPortal))
  (bind _returnvalue (Transformation|GetWorldLocation _portal))
  (bind _returnvalue_2 (Transformation|GetWorldRotation _portal))
  (bind _portal_2 (Variables|PortalBP_C|GetPortal _pair_portal))
  (bind _returnvalue_3 (Transformation|GetWorldLocation _portal_2))
  (bind _returnvalue_4 (Transformation|GetWorldRotation _portal_2))
  (bind _returnvalue_5 (Math|Transform|MakeTransform _returnvalue _returnvalue_2))
  (bind _returnvalue_6 (Math|Rotator|CombineRotators "0,180.000000, 0" _returnvalue_4))
  (bind _returnvalue_7 (Math|Transform|MakeTransform _returnvalue_3 _returnvalue_6))
  (return (Math|Transform|TransformLocation _returnvalue_7 (Math|Transform|InverseTransformLocation _returnvalue_5 (Transformation|GetWorldLocation Component))) (Math|Rotator|CombineRotators (Math|Rotator|CombineRotators (Transformation|GetWorldRotation Component) (Class|KismetMathLibrary|NegateRotator _returnvalue_2)) _returnvalue_6) (Math|Transform|TransformRotation _returnvalue_7 (Math|Transform|InverseTransformRotation _returnvalue_5 "0, 0, 0"))))

(fn ForceMinimumSpeed
  (params (InSpeed :type Vector))
  (return InSpeed))

(fn SpawnPortal
  (params (HitResult :type Hit%20Result%20Structure) (WasActive :type Boolean))
  (bind _returnvalue (Game|GetPlayerController 0))
  (bind (_bblockinghit _binitialoverlap _time _distance _location _impactpoint _normal _impactnormal) (Collision|BreakHitResult HitResult))
  (bind _returnvalue_2 (Math|Vector|VectorUp))
  (bind _self self)
  (bind _self_2 self)
  (bind _self_3 self)
  (bind _array (LocalVariables|GetArray))
  (bind _array_2 (LocalVariables|GetArray))
  (bind _chell (Variables|Default|GetChell))
  (bind _chell_2 (Variables|Default|GetChell))
  (bind _array_3 (LocalVariables|GetArray))
  (bind _array_4 (LocalVariables|GetArray))
  (bind _returnvalue_3 (Class|KismetMathLibrary|MakeRotfromYZ _impactnormal _returnvalue_2))
  (bind _returnvalue_4 (Controller|LineOfSightTo _returnvalue _self_3 "0, 0, 0" false))
  (bind _planeright (Variables|PortalBP_C|GetPlaneRight _self_2))
  (bind _defaultsceneroot (Variables|PortalBP_C|GetDefaultSceneRoot _self))
  (bind _defaultsceneroot_2 (Variables|PortalBP_C|GetDefaultSceneRoot _self_2))
  (bind _planetop (Variables|PortalBP_C|GetPlaneTop _self_2))
  (bind _planebottom (Variables|PortalBP_C|GetPlaneBottom _self_2))
  (bind _planeleft (Variables|PortalBP_C|GetPlaneLeft _self_2))
  (bind _outoverlappingcomponents (Class|PrimitiveComponent|GetOverlappingComponents _planeright))
  (bind _outoverlappingcomponents_2 (Class|PrimitiveComponent|GetOverlappingComponents _planeleft))
  (bind _outoverlappingcomponents_3 (Class|PrimitiveComponent|GetOverlappingComponents _planebottom))
  (bind _outoverlappingcomponents_4 (Class|PrimitiveComponent|GetOverlappingComponents _planetop))
  (bind _returnvalue_5 (Transformation|GetWorldLocation _defaultsceneroot_2))
  (bind _returnvalue_6 (Math|Vector|GetForwardVector _defaultsceneroot_2))
  (bind _returnvalue_7 (Math|Vector|GetUpVector _defaultsceneroot_2))
  ;[1 1 1] Initial Spawn
  (if (Variables|Default|GetIsBlue)
    (LocalVariables|SetSound "/Game/Portal/Portals/Audio/portal_blue.portal_blue")
    (else
      (LocalVariables|SetSound "/Game/Portal/Portals/Audio/portal_orange.portal_orange")))
  (bind _output_get (LocalVariables|SetBackupLocation (Transformation|GetWorldLocation _defaultsceneroot)))
  (LocalVariables|SetFixedLocation _output_get)
  (LocalVariables|SetBackupRotation (Transformation|GetWorldRotation _defaultsceneroot))
  (Transformation|SetActorLocationAndRotation _location _returnvalue_3)
  ;[1 1 1] Attempt Location Fix (Portals can't be half on wall)
  (Utilities|Array|Clear (LocalVariables|GetArray) :!label _label)
  (Utilities|Array|AddUnique _array_2 (Utilities|Array|Get(acopy) _outoverlappingcomponents))
  (if (Math|Boolean|ANDBoolean (== (Utilities|Array|Length _outoverlappingcomponents) 1) (== (Utilities|Array|Length _array_2) 1) _returnvalue_4)
    (Utilities|Array|AddUnique _array_3 (Utilities|Array|Get(acopy) _outoverlappingcomponents_2))
    (if (Math|Boolean|ANDBoolean (== (Utilities|Array|Length _outoverlappingcomponents_2) 1) (== (Utilities|Array|Length _array_3) 1) _returnvalue_4)
      (Utilities|Array|AddUnique _array_4 (Utilities|Array|Get(acopy) _outoverlappingcomponents_3))
      (if (Math|Boolean|ANDBoolean (== (Utilities|Array|Length _outoverlappingcomponents_3) 1) (== (Utilities|Array|Length _array_4) 1) _returnvalue_4)
        (Utilities|Array|AddUnique _array (Utilities|Array|Get(acopy) _outoverlappingcomponents_4))
        (if (Math|Boolean|ANDBoolean (== (Utilities|Array|Length _outoverlappingcomponents_4) 1) (== (Utilities|Array|Length _array) 1) _returnvalue_4)
          ;[1 1 1] Successful Spawn
          (Audio|SpawnSoundAttached (LocalVariables|GetSound) (Variables|/Game/Portal/FPC/Chell.Chell_C|GetCamera (Variables|Default|GetChell)) "None" "0, 0, 0" "0, 0, 0" "KeepRelativeOffset" false 0.5 1.0 0.0 0 0)
          (LocalVariables|SetAttempts 0)
          (CallFunction|Show self)
          (Default|ShowCrosshair _chell (Variables|/Game/Portal/FPC/Chell.Chell_C|GetCrosshairImages _chell))
          (else
            (LocalVariables|SetFixedLocation (+ _returnvalue_5 (Math|Vector|NegateVector _returnvalue_7)))
            (Transformation|SetActorLocationAndRotation _self_2 (stale _output_get_2) _returnvalue_3 :!label _label_2)
            (Math|Integer|IncrementInt (LocalVariables|GetAttempts)
              (:%20%20
                (if (< (LocalVariables|GetAttempts) 700)
                  (goto _label)
                  (else
                    ;[1 1 1] Cancel Spawn
                    (LocalVariables|SetAttempts 0)
                    (Transformation|SetActorLocationAndRotation _self_2 (LocalVariables|GetBackupLocation) (LocalVariables|GetBackupRotation))
                    (Audio|PlaySoundatLocation "/Game/Portal/Portals/Audio/error.error" (Transformation|GetWorldLocation (Variables|/Script/Engine.PlayerCameraManager|GetTransformComponent (Game|GetPlayerCameraManager 0))) "0, 0, 0" 1.0 1.0 0.0 0 0 0)
                    (if WasActive
                      (CallFunction|Show self))
                    (Default|ShowCrosshair _chell_2 (Variables|/Game/Portal/FPC/Chell.Chell_C|GetCrosshairImages _chell_2))))))))
        (else
          (LocalVariables|SetFixedLocation (+ _returnvalue_5 _returnvalue_7))
          (goto _label_2)))
      (else
        (LocalVariables|SetFixedLocation (+ _returnvalue_5 _returnvalue_6))
        (goto _label_2)))
    (else
      (bind _output_get_2 (LocalVariables|SetFixedLocation (+ _returnvalue_5 (Math|Vector|NegateVector _returnvalue_6))))
      (goto _label_2))))