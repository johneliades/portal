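; Portal gun Blueprint that fires a blue or orange portal shot, based on Portal.IsBlue.
; ShootPortal tints a dynamic energy material, brightens it by timeline, then line traces forward and spawns a BP_DarkEnergy projectile.
; A trace hit plays the color's sound, dims the material back to white and binds projectile impact.
; On impact, Portal spawns the portal using the earlier trace result, ignoring the projectile's hit.
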(event Custom|ShootPortal
  (bind _forward (Variables|Default|GetForward))
  (bind _portalgun (Variables|Default|GetPortalGun))
  (bind _returnvalue (Transformation|GetWorldLocation _forward))
  (bind _returnvalue_2 (Rendering|Material|CreateDynamicMaterialInstance (Variables|Default|GetPortalGun) 7 "/Game/Portal/Gun/M_Energy.M_Energy" "None" :!class /Script/Engine.PrimitiveComponent))
  (Variables|Default|SetEnergyMat _returnvalue_2)
  (if (Variables|/Game/Portal/Portals/BP_Portal.BP_Portal_C|GetIsBlue (Variables|Default|GetPortal))
    (bind _output_get (Variables|Default|SetPortalColor "(R=0.000000,G=254.999939,B=255.000000,A=1.000000)"))
    (Rendering|Material|SetVectorParameterValue (Variables|Default|GetEnergyMat) "Color" _output_get :!class /Script/Engine.MaterialInstanceDynamic)
    (bind _intensity (Timeline|Brighten PlayFromStart)
      (:Update
        (Rendering|Material|SetScalarParameterValue (Variables|Default|GetEnergyMat) "Intensity" _intensity :!class /Script/Engine.MaterialInstanceDynamic))
      (:Finished
        (bind (_outhit _returnvalue_3) (Collision|LineTraceByChannel _returnvalue (+ _returnvalue (* (Math|Vector|GetForwardVector _forward) 9999999)) "TraceTypeQuery1" false 0 "None" true (Variables|Default|GetPortalColor) (Variables|Default|GetPortalColor)))
        (bind _returnvalue_4 (Game|SpawnActorfromClass "/Game/Portal/Projectiles/BP_DarkEnergy.BP_DarkEnergy_C" (Transformation|GetWorldTransform _forward) "Undefined" "MultiplyWithRoot" self 2e+03 0))
        (if _returnvalue_3
          (if (Variables|/Game/Portal/Portals/BP_Portal.BP_Portal_C|GetIsBlue (Variables|Default|GetPortal))
            (Audio|SpawnSoundAttached "/Game/Portal/Portals/Audio/shoot_blue.shoot_blue" _portalgun "None" "0, 0, 0" "0, 0, 0" "KeepRelativeOffset" false 0.5 1.0 0.0 "/Game/Portal/LevelSounds/SoundAttenuation.SoundAttenuation" 0)
            (else
              (Audio|SpawnSoundAttached "/Game/Portal/Portals/Audio/shoot_orange.shoot_orange" _portalgun "None" "0, 0, 0" "0, 0, 0" "KeepRelativeOffset" false 0.5 1.0 0.0 "/Game/Portal/LevelSounds/SoundAttenuation.SoundAttenuation" 0)))
          (EventDispatchers|BindEventtoOnProjectileImpact _returnvalue_4 (delegate Custom|HitEvent))
          (bind _intensity_2 (Timeline|Dim ReverseFromEnd)
            (:Update
              (Rendering|Material|SetScalarParameterValue (Variables|Default|GetEnergyMat) "Intensity" _intensity_2 :!class /Script/Engine.MaterialInstanceDynamic))
            (:Finished
              (Rendering|Material|SetVectorParameterValue (Variables|Default|GetEnergyMat) "Color" "(R=1.000000,G=1.000000,B=1.000000,A=1.000000)" :!class /Script/Engine.MaterialInstanceDynamic))))))
    (else
      (bind _output_get_2 (Variables|Default|SetPortalColor "(R=255.000000,G=7.022327,B=0.000000,A=1.000000)"))
      (Rendering|Material|SetVectorParameterValue (Variables|Default|GetEnergyMat) "Color" _output_get_2 :!class /Script/Engine.MaterialInstanceDynamic)
      (Timeline|Brighten PlayFromStart))))

(event Custom|HitEvent
  (params (OtherActor :type Actor%20Object%20Reference) (Hit :type Hit%20Result%20Structure))
  (Default|SpawnPortal (Variables|Default|GetPortal) (stale Custom|ShootPortal _outhit)))

(event EventBeginPlay)

(event Collision|EventActorBeginOverlap
  (params (OtherActor :type Actor%20Object%20Reference)))

(event EventTick
  (params (DeltaSeconds :type Float%20%28single-precision%29)))

(fn ConstructionScript)