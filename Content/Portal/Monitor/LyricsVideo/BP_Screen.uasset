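; BP_Screen is a monitor actor that plays looping video with sound on an LED-style screen.
; PlayVideo puts the supplied video texture into a new M_LedScreen dynamic material on the SMP2Monitor mesh, then opens the media source on the supplied player.
; It also adds a half-volume media sound component at runtime for that player.
; StopVideo pauses the player and destroys that sound component.
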(event Custom|SetTexture
  (params (Texture :type Texture%20Object%20Reference))
  (bind _returnvalue (Rendering|Material|CreateDynamicMaterialInstance (Variables|Default|GetSM_P2Monitor) 1 "/Game/Portal/Monitor/M_LedScreen.M_LedScreen" "None" :!class /Script/Engine.PrimitiveComponent))
  (Rendering|Material|SetTextureParameterValue _returnvalue "PixelatedTexture" Texture))

(event Custom|PlayVideo
  (params (Player :type Media%20Player%20Object%20Reference) (VideoTexture :type Texture%20Object%20Reference) (MediaSource :type File%20Media%20Source%20Object%20Reference))
  (CallFunction|SetTexture VideoTexture)
  (Components|Timeline|SetLooping Player true)
  (bind _returnvalue (AddComponent|AddMediaSoundComponent false))
  (Audio|Components|Audio|SetVolumeMultiplier _returnvalue 0.5 :!class /Script/AudioMixer.SynthComponent)
  (Media|MediaSoundComponent|SetMediaPlayer _returnvalue Player)
  (Media|MediaPlayer|OpenSource Player MediaSource))

(event Custom|StopVideo
  (Sequencer|Player|Pause (stale Custom|PlayVideo Player))
  (Components|DestroyComponent (stale Custom|PlayVideo _returnvalue)))

(event EventBeginPlay)

(event Collision|EventActorBeginOverlap
  (params (OtherActor :type Actor%20Object%20Reference)))

(event EventTick
  (params (DeltaSeconds :type Float%20%28single-precision%29)))

(fn ConstructionScript)