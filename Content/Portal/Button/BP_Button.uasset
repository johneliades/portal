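; Portal-style floor button that opens its linked Gate while the player or any BPI_Interactable actor overlaps its box.
; An overlap counter triggers press and release only on the first entry and last exit, while interact messages notify overlapping actors.
; Each change toggles emissive glow and sound, and plays one animation forward or in reverse, with pressing resuming from the current position.
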(event OnComponentBeginOverlap(Box)
  (params (OverlappedComponent :type Primitive%20Component%20Object%20Reference) (OtherActor :type Actor%20Object%20Reference) (OtherComp :type Primitive%20Component%20Object%20Reference) (OtherBodyIndex :type Integer) (bFromSweep :type Boolean) (SweepResult :type Hit%20Result%20Structure%20%28by%20ref%29))
  (bind _button (Variables|Default|GetButton))
  (Class|BPIInteractable|OnInteract(Message) OtherActor)
  (bind _output_get (Variables|Default|SetPosition (Class|SkeletalMeshComponent|GetPosition _button)))
  (if (or (== OtherActor (Game|GetPlayerCharacter 0)) (Utilities|DoesObjectImplementInterface OtherActor "/Game/Portal/Cubes/BPI_Interactable.BPI_Interactable_C"))
    (Math|Integer|IncrementInt (Variables|Default|GetCounter)
      (:%20%20
        (if (== (Variables|Default|GetCounter) 1)
          (Rendering|Material|SetScalarParameterValueonMaterials (Variables|Default|GetButton) "EmissiveStrength4" 6.4)
          (Components|Animation|PlayAnimation _button "/Game/Portal/Button/AS_button_-_from_portal_2_original_Skeleton_Sequence1.AS_button_-_from_portal_2_original_Skeleton_Sequence1" false)
          (Audio|Components|Audio|Stop _button)
          (Components|Animation|SetPosition _button _output_get true)
          (Audio|SpawnSoundAttached "/Game/Portal/Button/Audio/portal_button_down_01.portal_button_down_01" (Variables|Default|GetDefaultSceneRoot) "None" "0, 0, 0" "0, 0, 0" "KeepRelativeOffset" false 0.15 1.0 0.0 "/Game/Portal/LevelSounds/SoundAttenuation.SoundAttenuation" 0)
          (Components|Timeline|SetPlayRate (Variables|Default|GetButton) 1.3)
          (Audio|Components|Audio|Play (Variables|Default|GetButton) false)
          (Default|OpenGate (Variables|Default|GetGate)))))))

(event OnComponentEndOverlap(Box)
  (params (OverlappedComponent :type Primitive%20Component%20Object%20Reference) (OtherActor :type Actor%20Object%20Reference) (OtherComp :type Primitive%20Component%20Object%20Reference) (OtherBodyIndex :type Integer))
  (if (or (Utilities|DoesObjectImplementInterface OtherActor "/Game/Portal/Cubes/BPI_Interactable.BPI_Interactable_C") (== OtherActor (Game|GetPlayerCharacter 0)))
    (Class|BPIInteractable|OnEndInteract(Message) OtherActor)
    (Math|Integer|DecrementInt (Variables|Default|GetCounter)
      (:%20%20
        (if (== (Variables|Default|GetCounter) 0)
          (Rendering|Material|SetScalarParameterValueonMaterials (Variables|Default|GetButton) "EmissiveStrength4" 0.0)
          (Audio|SpawnSoundAttached "/Game/Portal/Button/Audio/portal_button_up_01.portal_button_up_01" (Variables|Default|GetDefaultSceneRoot) "None" "0, 0, 0" "0, 0, 0" "KeepRelativeOffset" false 0.15 1.0 0.0 "/Game/Portal/LevelSounds/SoundAttenuation.SoundAttenuation" 0)
          (Components|Timeline|SetPlayRate (Variables|Default|GetButton) -1.3)
          (Audio|Components|Audio|Play (Variables|Default|GetButton) false)
          (Default|CloseGate (Variables|Default|GetGate)))))))

(fn ConstructionScript)