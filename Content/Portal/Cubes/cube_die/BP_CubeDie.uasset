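; BP_CubeDie is a cube actor, under the Portal cubes folder, that lights up while it is interacted with.
; On BeginPlay it creates two dynamic material instances and assigns them to two material slots of its Cube mesh.
; The interact and end-interact events raise and reset the Intensity scalar parameter on both instances, toggling the effect.
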(event EventBeginPlay
  (bind _returnvalue (Rendering|Material|CreateDynamicMaterialInstance "/Game/Portal/Cubes/cube_die/M_Material__49.M_Material__49" "None" "None" :!class /Script/Engine.KismetMaterialLibrary))
  (Rendering|Material|SetMaterial (Variables|Default|GetCube) 4 _returnvalue)
  (bind _returnvalue_2 (Rendering|Material|CreateDynamicMaterialInstance "/Game/Portal/Cubes/cube_die/M_Material__48_ncl1_2.M_Material__48_ncl1_2" "None" "None" :!class /Script/Engine.KismetMaterialLibrary))
  (Rendering|Material|SetMaterial (Variables|Default|GetCube) 5 _returnvalue_2))

(event EventOnInteract
  (params (Component :type Primitive%20Component%20Object%20Reference))
  (Rendering|Material|SetScalarParameterValue (stale EventBeginPlay _returnvalue) "Intensity" 0.1 :!class /Script/Engine.MaterialInstanceDynamic)
  (Rendering|Material|SetScalarParameterValue (stale EventBeginPlay _returnvalue_2) "Intensity" 0.1 :!class /Script/Engine.MaterialInstanceDynamic))

(event EventOnEndInteract
  (params (Component :type Primitive%20Component%20Object%20Reference))
  (Rendering|Material|SetScalarParameterValue (stale EventBeginPlay _returnvalue) "Intensity" 0.0 :!class /Script/Engine.MaterialInstanceDynamic)
  (Rendering|Material|SetScalarParameterValue (stale EventBeginPlay _returnvalue_2) "Intensity" 0.0 :!class /Script/Engine.MaterialInstanceDynamic))

(fn ConstructionScript)