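; BP_CubeHeart is a heart cube Blueprint in the Portal content that changes its material while being interacted with.
; On the first interaction it caches all materials of the passed component, and on every interaction it swaps slot 0 to a fixed material.
; When interaction ends, it reapplies the cached materials to the passed component by slot index.
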(event EventOnInteract
  (params (Component :type Primitive%20Component%20Object%20Reference))
  (Utilities|FlowControl|Sequence
    (:then_0
      (Utilities|FlowControl|DoOnce false
        (:Completed
          (bind _index (Utilities|FlowControl|ForLoopwithBreak 0 (Rendering|Material|GetNumMaterials Component))
            (:LoopBody
              (Utilities|Array|Add (Variables|Default|GetMaterialBackup) (Rendering|Material|GetMaterial Component _index)))))))
    (:then_1
      (Rendering|Material|SetMaterial Component 0 "/Game/Portal/Cubes/cube_heart/M_45801d2e_dds.M_45801d2e_dds"))))

(event EventOnEndInteract
  (params (Component :type Primitive%20Component%20Object%20Reference))
  (for (_array_element _array_index) (Variables|Default|GetMaterialBackup)
    (Rendering|Material|SetMaterial Component _array_index _array_element)))

(fn ConstructionScript)